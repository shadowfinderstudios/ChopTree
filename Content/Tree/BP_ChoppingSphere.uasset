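; BP_ChoppingSphere is a sphere actor that marks a dissolve area on procedural meshes it touches, apparently for tree chopping.
; On begin overlap with an actor that has a ProceduralMeshComponent, it writes the sphere's position in that mesh's local space and its scaled size to MPC_DissolveArea.
; The parameter collection is global, so each qualifying overlap overwrites the previous area.
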(event `self.ReceiveActorBeginOverlap`
  (params (OtherActor :type "Actor Object Reference"))
  (bind _returnvalue (`self.GetComponentByClass` OtherActor "/Script/ProceduralMeshComponent.ProceduralMeshComponent"))
  (bind _sphere (`self.Sphere`))
  (bind _returnvalue_x (`KismetMathLibrary.BreakVector` (`SceneComponent.K2_GetComponentScale` _sphere)))
  (`/Engine/EditorBlueprintResources/StandardMacros.IsValid` _returnvalue
    (:`Is Valid`
      (`KismetMaterialLibrary.SetVectorParameterValue` "/Game/Tree/MPC_DissolveArea.MPC_DissolveArea" "location" (`KismetMathLibrary.Conv_VectorToLinearColor` (`KismetMathLibrary.InverseTransformLocation` (`SceneComponent.K2_GetComponentToWorld` _returnvalue) (`SceneComponent.K2_GetComponentLocation` _sphere))))
      (`KismetMaterialLibrary.SetScalarParameterValue` "/Game/Tree/MPC_DissolveArea.MPC_DissolveArea" "scale" (* _returnvalue_x 100.0)))))

(fn `UserConstructionScript`)